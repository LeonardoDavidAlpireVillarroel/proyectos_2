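; BP_CurveSpline is an actor that locks the third-person character onto a curved spline path.
; While active, Tick snaps the capsule's X/Y to the closest spline point and keeps its Z.
; SplineBegin overlaps start or end the lock by X velocity, updating the player's spline state and reference.
; BeginPlay aligns SplineEnd to the spline, but its overlap logic is disconnected.
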(event OnComponentBeginOverlap(SplineBegin)
  (params (OverlappedComponent :type Primitive%20Component%20Object%20Reference) (OtherActor :type Actor%20Object%20Reference) (OtherComp :type Primitive%20Component%20Object%20Reference) (OtherBodyIndex :type Integer) (bFromSweep :type Boolean) (SweepResult :type Hit%20Result%20Structure%20%28by%20ref%29))
  (bind _playerref (Variables|Default|GetPlayerRef))
  (if (== OtherActor _playerref)
    (if (< (.x (Variables|/Script/Engine.MovementComponent|GetVelocity (Variables|/Script/Engine.Character|GetCharacterMovement _playerref))) 1.5e+02)
      (CallFunction|BeginSPline)
      (else
        (CallFunction|EndSpline)))))

(event OnComponentBeginOverlap(SplineEnd)
  (params (OverlappedComponent :type Primitive%20Component%20Object%20Reference) (OtherActor :type Actor%20Object%20Reference) (OtherComp :type Primitive%20Component%20Object%20Reference) (OtherBodyIndex :type Integer) (bFromSweep :type Boolean) (SweepResult :type Hit%20Result%20Structure%20%28by%20ref%29)))

(event Custom|BeginSPline
  (bind _playerref (Variables|Default|GetPlayerRef))
  ;[1 1 1] Begin and end Spline
  (Variables|/Game/ThirdPerson/Blueprints/BP_ThirdPersonCharacter.BP_ThirdPersonCharacter_C|SetInSpline _playerref true)
  (Variables|/Game/ThirdPerson/Blueprints/BP_ThirdPersonCharacter.BP_ThirdPersonCharacter_C|SetCurveSplineRef\ _playerref self)
  (Transformation|SetWorldLocation (Variables|/Script/Engine.Character|GetCapsuleComponent (Variables|Default|GetPlayerRef)) (Spline|FindLocationClosesttoWorldLocation (Variables|Default|GetSpline) (Transformation|GetWorldLocation (Variables|/Script/Engine.Character|GetCapsuleComponent (Variables|Default|GetPlayerRef))) "World") false false)
  (Variables|Default|SetStratTick true))

(event Custom|EndSpline
  (bind _playerref (Variables|Default|GetPlayerRef))
  ;[1 1 1] Begin and end Spline
  (Variables|/Game/ThirdPerson/Blueprints/BP_ThirdPersonCharacter.BP_ThirdPersonCharacter_C|SetInSpline _playerref false)
  (Variables|/Game/ThirdPerson/Blueprints/BP_ThirdPersonCharacter.BP_ThirdPersonCharacter_C|SetCurveSplineRef\ _playerref 0)
  (Variables|Default|SetStratTick false))

(event EventBeginPlay
  (bind _splineend (Variables|Default|GetSplineEnd))
  (bind _splineend_2 (Variables|Default|GetSplineEnd))
  (bind _spline (Variables|Default|GetSpline))
  (bind _spline_2 (Variables|Default|GetSpline))
  (bind _returnvalue (Transformation|GetWorldLocation _splineend))
  (bind _returnvalue_2 (Spline|FindLocationClosesttoWorldLocation _spline _returnvalue "World"))
  (bind (_x _y _z) (Math|Vector|BreakVector _returnvalue_2))
  ;[1 1 1] BeginPlay
  (Transformation|SetWorldLocation _splineend_2 (Math|Vector|MakeVector _x (+ _y 5e+01) _z) false false)
  (Transformation|SetWorldRotation _splineend_2 (Spline|GetRotationatSplinePoint _spline_2 (Spline|GetNumberOfSplinePoints _spline_2) "Local") false false)
  (Variables|Default|SetPlayerRef (.AsBP%20Third%20Person%20Character (Utilities|Casting|CastToBP_ThirdPersonCharacter (Game|GetPlayerCharacter 0)))))

(event EventTick
  (params (DeltaSeconds :type Float%20%28single-precision%29))
  (bind _spline (Variables|Default|GetSpline))
  (bind _playerref (Variables|Default|GetPlayerRef))
  (bind _capsulecomponent (Variables|/Script/Engine.Character|GetCapsuleComponent _playerref))
  (bind _returnvalue (Transformation|GetWorldLocation _capsulecomponent))
  (bind _returnvalue_2 (Spline|FindLocationClosesttoWorldLocation _spline _returnvalue "World"))
  (if (Variables|Default|GetStratTick)
    (Transformation|SetWorldLocation (Variables|/Script/Engine.Character|GetCapsuleComponent (Variables|Default|GetPlayerRef)) (Math|Vector|MakeVector (.x _returnvalue_2) (.y _returnvalue_2) (.Z (Math|Vector|BreakVector _returnvalue))) false false)))

(fn ConstructionScript)
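; Trigger actor for the transition cinematic between level 1 and level 2.
; When BP_ThirdPersonCharacter enters its Box, it hands the character a reference to itself and sets Dentro, which clears on exit.
; Its PlayCinematic event, not called within this Blueprint, creates a player for LS_Nivel1a2 and starts the sequence.
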(event OnComponentEndOverlap(Box)
  (params (OverlappedComponent :type Primitive%20Component%20Object%20Reference) (OtherActor :type Actor%20Object%20Reference) (OtherComp :type Primitive%20Component%20Object%20Reference) (OtherBodyIndex :type Integer))
  (Utilities|Casting|CastToBP_ThirdPersonCharacter OtherActor)
  (Variables|Default|Setdentro? false))

(event OnComponentBeginOverlap(Box)
  (params (OverlappedComponent :type Primitive%20Component%20Object%20Reference) (OtherActor :type Actor%20Object%20Reference) (OtherComp :type Primitive%20Component%20Object%20Reference) (OtherBodyIndex :type Integer) (bFromSweep :type Boolean) (SweepResult :type Hit%20Result%20Structure%20%28by%20ref%29))
  (bind _asbp_third_person_character (Utilities|Casting|CastToBP_ThirdPersonCharacter OtherActor))
  (Variables|/Game/ThirdPerson/Blueprints/BP_ThirdPersonCharacter.BP_ThirdPersonCharacter_C|SetBP_TransicionN1a2 _asbp_third_person_character self)
  (Variables|Default|Setdentro? true))

(event Custom|PlayCinematic
  (Sequencer|Player|CreateLevelSequencePlayer "/Game/MyBlueprints/Transiciones/LS_Nivel1a2.LS_Nivel1a2")
  (Sequencer|Player|Play (Variables|/Script/LevelSequence.LevelSequenceActor|GetSequencePlayer (Variables|Default|GetLevelSequence)) :!class /Script/MovieScene.MovieSceneSequencePlayer))

(event EventBeginPlay)

(event Collision|EventActorBeginOverlap
  (params (OtherActor :type Actor%20Object%20Reference)))

(event EventTick
  (params (DeltaSeconds :type Float%20%28single-precision%29)))

(fn ConstructionScript)
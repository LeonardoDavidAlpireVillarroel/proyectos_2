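; Canned snack pickup that restores the player character's hunger and then destroys itself.
; The Interact volume toggles input and the E prompt, so pressing Interactuar consumes the snack after a short delay.
; A larger-purpose Box volume resets and reveals the SmellSnack effect when the player enters.
; On exit, if HaVistoElRecuerdo is set, a Timeline lerp moves the smell effect downward.
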(event OnComponentBeginOverlap(Interact)
  (params (OverlappedComponent :type Primitive%20Component%20Object%20Reference) (OtherActor :type Actor%20Object%20Reference) (OtherComp :type Primitive%20Component%20Object%20Reference) (OtherBodyIndex :type Integer) (bFromSweep :type Boolean) (SweepResult :type Hit%20Result%20Structure%20%28by%20ref%29))
  (Utilities|Casting|CastToBP_ThirdPersonCharacter OtherActor)
  (Input|EnableInput (Game|GetPlayerController 0))
  (Development|SetHiddeninGame (Variables|Default|GetE) false false))

(event OnComponentEndOverlap(Interact)
  (params (OverlappedComponent :type Primitive%20Component%20Object%20Reference) (OtherActor :type Actor%20Object%20Reference) (OtherComp :type Primitive%20Component%20Object%20Reference) (OtherBodyIndex :type Integer))
  (Utilities|Casting|CastToBP_ThirdPersonCharacter OtherActor)
  (Input|DisableInput (Game|GetPlayerController 0))
  (Development|SetHiddeninGame (Variables|Default|GetE) true false))

(event OnComponentBeginOverlap(Box)
  (params (OverlappedComponent :type Primitive%20Component%20Object%20Reference) (OtherActor :type Actor%20Object%20Reference) (OtherComp :type Primitive%20Component%20Object%20Reference) (OtherBodyIndex :type Integer) (bFromSweep :type Boolean) (SweepResult :type Hit%20Result%20Structure%20%28by%20ref%29))
  (bind _smell_snack (Variables|Default|GetSmell_Snack))
  ;[1 1 1] Aparece y desaparece el olor
  (Utilities|Casting|CastToBP_ThirdPersonCharacter OtherActor)
  (Niagara|ResetSystem _smell_snack)
  (Development|SetHiddeninGame _smell_snack false false))

(event OnComponentEndOverlap(Box)
  (params (OverlappedComponent :type Primitive%20Component%20Object%20Reference) (OtherActor :type Actor%20Object%20Reference) (OtherComp :type Primitive%20Component%20Object%20Reference) (OtherBodyIndex :type Integer))
  (bind _smell_snack (Variables|Default|GetSmell_Snack))
  (bind _returnvalue (Transformation|GetWorldLocation _smell_snack))
  ;[1 1 1] Aparece y desaparece el olor
  (Utilities|Casting|CastToBP_ThirdPersonCharacter OtherActor)
  (if (Variables|Default|GetHaVistoElRecuerdo?)
    (bind _newtrack_0 (Timeline|Timeline Play)
      (:Update
        (Transformation|SetWorldLocation _smell_snack (Math|Vector|Lerp(Vector) (Math|Vector|MakeVector (.x _returnvalue) (.y _returnvalue) (.z _returnvalue)) (Math|Vector|MakeVector (.x _returnvalue) (.y _returnvalue) (+ (.z _returnvalue) -1e+02)) _newtrack_0) false false)))))

(event Input|ActionEvents|InputActionInteractuar
  (params (Key :type Key%20Structure :default "None"))
  (:Pressed
    (Utilities|FlowControl|Delay 2.0)
    (Default|RecuperarHambre (.AsBP%20Third%20Person%20Character (Utilities|Casting|CastToBP_ThirdPersonCharacter (Game|GetPlayerCharacter 0))))
    (Actor|DestroyActor)))

(fn ConstructionScript)
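; BP_Recuerdo1 is an interactable memory ("recuerdo") pickup that shows the Recuerdo1 image-viewer widget to the player.
; The Interact volume toggles input and the E prompt; Interactuar opens the widget after a delay, switches to UI-only input and sets TimePause on the character.
; The ViewSmell volume restarts and reveals the Smell effect, which a timeline sinks downward on exit once the memory has been seen.
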(event OnComponentBeginOverlap(Interact)
  (params (OverlappedComponent :type Primitive%20Component%20Object%20Reference) (OtherActor :type Actor%20Object%20Reference) (OtherComp :type Primitive%20Component%20Object%20Reference) (OtherBodyIndex :type Integer) (bFromSweep :type Boolean) (SweepResult :type Hit%20Result%20Structure%20%28by%20ref%29))
  ;[1 1 1] Aparece y desaparece el boton E
  (Utilities|Casting|CastToBP_ThirdPersonCharacter OtherActor)
  (Input|EnableInput (Game|GetPlayerController 0))
  (Development|SetHiddeninGame (Variables|Default|GetE) false false)
  (Variables|Default|SetDentroDeRango? true))

(event OnComponentEndOverlap(Interact)
  (params (OverlappedComponent :type Primitive%20Component%20Object%20Reference) (OtherActor :type Actor%20Object%20Reference) (OtherComp :type Primitive%20Component%20Object%20Reference) (OtherBodyIndex :type Integer))
  ;[1 1 1] Aparece y desaparece el boton E
  (Utilities|Casting|CastToBP_ThirdPersonCharacter OtherActor)
  (Input|DisableInput (Game|GetPlayerController 0))
  (Development|SetHiddeninGame (Variables|Default|GetE) true false)
  (Variables|Default|SetDentroDeRango? false))

(event OnComponentBeginOverlap(ViewSmell)
  (params (OverlappedComponent :type Primitive%20Component%20Object%20Reference) (OtherActor :type Actor%20Object%20Reference) (OtherComp :type Primitive%20Component%20Object%20Reference) (OtherBodyIndex :type Integer) (bFromSweep :type Boolean) (SweepResult :type Hit%20Result%20Structure%20%28by%20ref%29))
  (bind _smell (Variables|Default|GetSmell))
  ;[1 1 1] Aparece y desaparece el olor
  (Utilities|Casting|CastToBP_ThirdPersonCharacter OtherActor)
  (Niagara|ResetSystem _smell)
  (Development|SetHiddeninGame _smell false false))

(event OnComponentEndOverlap(ViewSmell)
  (params (OverlappedComponent :type Primitive%20Component%20Object%20Reference) (OtherActor :type Actor%20Object%20Reference) (OtherComp :type Primitive%20Component%20Object%20Reference) (OtherBodyIndex :type Integer))
  (bind _smell (Variables|Default|GetSmell))
  (bind _returnvalue (Transformation|GetWorldLocation _smell))
  ;[1 1 1] Aparece y desaparece el olor
  (Utilities|Casting|CastToBP_ThirdPersonCharacter OtherActor)
  (if (Variables|Default|GetHaVistoElRecuerdo?)
    (bind _newtrack_0 (Timeline|Timeline PlayFromStart)
      (:Update
        (Transformation|SetWorldLocation _smell (Math|Vector|Lerp(Vector) (Math|Vector|MakeVector (.x _returnvalue) (.y _returnvalue) (.z _returnvalue)) (Math|Vector|MakeVector (.x _returnvalue) (.y _returnvalue) (+ (.z _returnvalue) -1e+02)) _newtrack_0) false false)))))

(event Input|ActionEvents|InputActionInteractuar
  (params (Key :type Key%20Structure :default "None"))
  (bind _returnvalue (Game|GetPlayerController 0))
  ;[1 1 1] Visor de imagen
  (:Pressed
    (if (Variables|Default|GetDentroDeRango?)
      (Utilities|FlowControl|Delay 2.0)
      (bind _returnvalue_2 (UserInterface|CreateWidget "/Game/MyBlueprints/Interfaz/Recuerdo1.Recuerdo1_C" _returnvalue))
      (UserInterface|Viewport|AddtoViewport _returnvalue_2 0)
      (Input|SetInputModeUIOnly _returnvalue _returnvalue_2 "DoNotLock" false)
      (Variables|/Script/Engine.PlayerController|SetbShowMouseCursor _returnvalue true)
      (Variables|/Game/ThirdPerson/Blueprints/BP_ThirdPersonCharacter.BP_ThirdPersonCharacter_C|SetTimePause? (.AsBP%20Third%20Person%20Character (Utilities|Casting|CastToBP_ThirdPersonCharacter (Game|GetPlayerCharacter 0))) true)
      (Variables|Default|SetHaVistoElRecuerdo? true))))

(fn ConstructionScript)
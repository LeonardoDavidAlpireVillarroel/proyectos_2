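; BP_EnemyBase is a hunter enemy that chases the player and costs them a life when it catches them.
; PawnSensing raises walk speed on seeing any pawn and starts an AIMoveTo toward player 0, regardless of who was seen.
; A successful move calls MuerteSpawn and PerderVida on the player's BP_ThirdPersonCharacter.
; BeginPlay stores the spawn location, but the nodes to return there and restore slower speed are disconnected.
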(event OnSeePawn(PawnSensing)
  (params (Pawn :type Pawn%20Object%20Reference))
  (Variables|/Script/Engine.CharacterMovementComponent|SetMaxWalkSpeed (Variables|Character|GetCharacterMovement) 6e+02)
  (CallFunction|SeguirPersonaje))

(event Custom|Seguir%20personaje
  (AI|AIMoveTo self "0, 0, 0" (Game|GetPlayerCharacter 0) 1.5e+02 false
    (:OnSuccess
      (bind _asbp_third_person_character (Utilities|Casting|CastToBP_ThirdPersonCharacter (Game|GetPlayerCharacter 0)))
      (Default|MuerteSpawn _asbp_third_person_character)
      (Default|PerderVida _asbp_third_person_character))))

(event EventBeginPlay
  (Variables|Default|SetEnemySpawn (Transformation|GetActorLocation self)))

(fn ConstructionScript)
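; BP_Female is a hostile female character that costs the player a life, via PerderVida on BP_ThirdPersonCharacter, when its capsule begins an overlap with them.
; When PawnSensing sees a pawn, it raises its walk speed for a few seconds, then lowers it.
; A DoOnce plays the scare sound at its location on sighting and re-arms after that delay, preventing repeats during the burst.
; The graph contains no movement or chase logic.
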(event OnSeePawn(PawnSensing)
  (params (Pawn :type Pawn%20Object%20Reference))
  (Utilities|FlowControl|Sequence
    (:then_0
      (Variables|/Script/Engine.CharacterMovementComponent|SetMaxWalkSpeed (Variables|Character|GetCharacterMovement) 6.5e+02)
      (Utilities|FlowControl|Delay 5.0)
      (Variables|/Script/Engine.CharacterMovementComponent|SetMaxWalkSpeed (Variables|Character|GetCharacterMovement) 2e+02)
      (goto _label Reset))
    (:then_1
      (Utilities|FlowControl|DoOnce false :!label _label
        (:Completed
          (Audio|PlaySoundatLocation "/Game/MyBlueprints/Sonidos/susto_mujer.susto_mujer" (Transformation|GetWorldLocation (Variables|Collision|GetCapsuleComponent)) "0, 0, 0" 1.0 1.0 0.0 0 0 0 0))))))

(event OnComponentBeginOverlap(Capsule)
  (params (OverlappedComponent :type Primitive%20Component%20Object%20Reference) (OtherActor :type Actor%20Object%20Reference) (OtherComp :type Primitive%20Component%20Object%20Reference) (OtherBodyIndex :type Integer) (bFromSweep :type Boolean) (SweepResult :type Hit%20Result%20Structure%20%28by%20ref%29))
  (Default|PerderVida (.AsBP%20Third%20Person%20Character (Utilities|Casting|CastToBP_ThirdPersonCharacter OtherActor))))

(fn ConstructionScript)